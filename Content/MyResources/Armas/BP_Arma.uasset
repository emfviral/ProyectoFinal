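; Weapon actor that the player can equip, drop, holster and switch, receiving input enabled by overlapping its collision and disabled on overlap end.
; Equipar snaps it to the character's hand socket and sets ArmedBP and CurrentWeapon; Soltar detaches it.
; Mantener moves the current weapon to its SecondaryWeapon socket.
; Seleccionar holsters, then draws attached actor index 1 for both Long and Short; a FlipFlop alternates the two calls.
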(event OnComponentBeginOverlap(Colision)
  (params (OverlappedComponent :type Primitive%20Component%20Object%20Reference) (OtherActor :type Actor%20Object%20Reference) (OtherComp :type Primitive%20Component%20Object%20Reference) (OtherBodyIndex :type Integer) (bFromSweep :type Boolean) (SweepResult :type Hit%20Result%20Structure%20%28by%20ref%29))
  ;[1 1 1] Se activa cuando tengo armas
  (CallFunction|InputEnable true))

(event OnComponentEndOverlap(Colision)
  (params (OverlappedComponent :type Primitive%20Component%20Object%20Reference) (OtherActor :type Actor%20Object%20Reference) (OtherComp :type Primitive%20Component%20Object%20Reference) (OtherBodyIndex :type Integer))
  ;[1 1 1] Se desactiva el teclado cuando no tengo armas
  (bind _asthird_person_character (Utilities|Casting|CastToThirdPersonCharacter (Game|GetPlayerCharacter 0)))
  (if (Variables|/Game/ThirdPersonBP/Blueprints/ThirdPersonCharacter.ThirdPersonCharacter_C|GetArmed_BP _asthird_person_character)
    _
    (else
      _))
  (CallFunction|InputEnable false))

(event EventBeginPlay)

(event Collision|EventActorBeginOverlap
  (params (OtherActor :type Actor%20Object%20Reference)))

(event EventTick
  (params (DeltaSeconds :type Float%20%28single-precision%29)))

(event Input|ActionEvents|InputActionEquipar
  (params (Key :type Key%20Structure :default "None"))
  ;[1 1 1] Equipar (E)
  (:Pressed
    (CallFunction|Equipar)))

(event Input|ActionEvents|InputActionSoltar
  (params (Key :type Key%20Structure :default "None"))
  (:Pressed
    (CallFunction|Soltar)))

(event Input|ActionEvents|InputActionMantener
  (params (Key :type Key%20Structure :default "None"))
  (:Pressed
    (CallFunction|Mantener)))

(event Input|ActionEvents|InputActionPrimaria
  (params (Key :type Key%20Structure :default "None"))
  ;[1 1 1] Intercambio de Armas
  (:Pressed
    (CallFunction|Seleccionar "Long")))

(event Input|ActionEvents|InputActionSecundaria
  (params (Key :type Key%20Structure :default "None"))
  ;[1 1 1] Intercambio de Armas
  (:Pressed
    (CallFunction|Seleccionar "Short")))

(event Input|ActionEvents|InputActionIntercambio
  (params (Key :type Key%20Structure :default "None"))
  ;[1 1 1] Intercambio de Armas
  (:Pressed
    (Utilities|FlowControl|FlipFlop
      (:A
        (CallFunction|Seleccionar "Long"))
      (:B
        (CallFunction|Seleccionar "Short")))))

(fn ConstructionScript)

(fn Equipar
  (params (PlayerIndex :type Integer))
  (bind _returnvalue (Game|GetPlayerCharacter 0))
  ;[1 1 1] EQUIPAR SIMPLE
  (Transformation|AttachComponentToComponent self (Variables|/Script/Engine.Character|GetMesh _returnvalue) "Weapon_Socket" "SnapToTarget" "SnapToTarget" "SnapToTarget" true)
  (bind _asthird_person_character (Utilities|Casting|CastToThirdPersonCharacter _returnvalue))
  (Variables|/Game/ThirdPersonBP/Blueprints/ThirdPersonCharacter.ThirdPersonCharacter_C|SetArmed_BP _asthird_person_character true)
  (Variables|/Game/ThirdPersonBP/Blueprints/ThirdPersonCharacter.ThirdPersonCharacter_C|SetCurrent_Weapon _asthird_person_character self)
  (Collision|SetCollisionEnabled (Variables|Default|GetColision) "NoCollision"))

(fn Soltar
  (params (Arma :type BP%20Arma%20Object%20Reference))
  (bind _asthird_person_character (Utilities|Casting|CastToThirdPersonCharacter (Game|GetPlayerCharacter 0)))
  (Variables|/Game/ThirdPersonBP/Blueprints/ThirdPersonCharacter.ThirdPersonCharacter_C|SetArmed_BP _asthird_person_character false)
  (Variables|/Game/ThirdPersonBP/Blueprints/ThirdPersonCharacter.ThirdPersonCharacter_C|SetCurrent_Weapon _asthird_person_character 0)
  (Utilities|IsValid Arma
    (:Is%20Valid
      (Transformation|DetachFromActor "KeepWorld" "KeepWorld" "KeepWorld")
      (Collision|SetCollisionEnabled (Variables|Default|GetColision) "NoCollision"))
    (:Is%20Not%20Valid
      (Transformation|DetachFromActor "KeepWorld" "KeepWorld" "KeepWorld")
      (Collision|SetCollisionEnabled (Variables|Default|GetColision) "NoCollision"))))

(fn InputEnable
  (params (Enable :type Boolean))
  (bind _returnvalue (Game|GetPlayerController 0))
  ;[1 1 1] Activa o Desactiva teclas del jugador
  (if Enable
    (Input|EnableInput _returnvalue)
    (else
      (Input|DisableInput _returnvalue))))

(fn Mantener
  (bind _returnvalue (Game|GetPlayerCharacter 0))
  (bind _asthird_person_character (Utilities|Casting|CastToThirdPersonCharacter _returnvalue))
  (Utilities|IsValid (Variables|/Game/ThirdPersonBP/Blueprints/ThirdPersonCharacter.ThirdPersonCharacter_C|GetCurrent_Weapon _asthird_person_character)
    (:Is%20Valid
      (Transformation|AttachComponentToComponent (Variables|/Game/ThirdPersonBP/Blueprints/ThirdPersonCharacter.ThirdPersonCharacter_C|GetCurrent_Weapon _asthird_person_character) (Variables|/Script/Engine.Character|GetMesh _returnvalue) (Variables|BP_Arma_C|GetSecondary_Weapon (Variables|/Game/ThirdPersonBP/Blueprints/ThirdPersonCharacter.ThirdPersonCharacter_C|GetCurrent_Weapon _asthird_person_character)) "SnapToTarget" "SnapToTarget" "SnapToTarget" true)
      (Variables|/Game/ThirdPersonBP/Blueprints/ThirdPersonCharacter.ThirdPersonCharacter_C|SetArmed_BP _asthird_person_character false)
      (Variables|/Game/ThirdPersonBP/Blueprints/ThirdPersonCharacter.ThirdPersonCharacter_C|SetCurrent_Weapon _asthird_person_character 0))))

(fn Seleccionar
  (params (TipoDeArma :type String))
  (bind _returnvalue (Game|GetPlayerCharacter 0))
  (bind _primary_weapon (Variables|Default|GetPrimary_Weapon))
  (CallFunction|Mantener)
  (bind _asthird_person_character (Utilities|Casting|CastToThirdPersonCharacter _returnvalue))
  (LocalVariables|SetTPC _asthird_person_character)
  (LocalVariables|SetTPC_MESH (Variables|/Script/Engine.Character|GetMesh _returnvalue))
  (if (Utilities|Enum|Equal(Enum) TipoDeArma "Long")
    (bind _asbp_arma (Utilities|Casting|CastToBP_Arma (Utilities|Array|Get(acopy) (Actor|GetAttachedActors (LocalVariables|GetTPC) true) 1)))
    (Transformation|AttachComponentToComponent _asbp_arma (LocalVariables|GetTPC_MESH) _primary_weapon "SnapToTarget" "SnapToTarget" "SnapToTarget" true)
    (Variables|/Game/ThirdPersonBP/Blueprints/ThirdPersonCharacter.ThirdPersonCharacter_C|SetCurrent_Weapon (LocalVariables|GetTPC) _asbp_arma)
    (else
      (bind _asbp_arma_2 (Utilities|Casting|CastToBP_Arma (Utilities|Array|Get(acopy) (Actor|GetAttachedActors (LocalVariables|GetTPC) true) 1)))
      (Transformation|AttachComponentToComponent _asbp_arma_2 (LocalVariables|GetTPC_MESH) _primary_weapon "SnapToTarget" "SnapToTarget" "SnapToTarget" true)
      (Variables|/Game/ThirdPersonBP/Blueprints/ThirdPersonCharacter.ThirdPersonCharacter_C|SetCurrent_Weapon (LocalVariables|GetTPC) _asbp_arma_2)))
  (Variables|/Game/ThirdPersonBP/Blueprints/ThirdPersonCharacter.ThirdPersonCharacter_C|SetArmed_BP (LocalVariables|GetTPC) true))